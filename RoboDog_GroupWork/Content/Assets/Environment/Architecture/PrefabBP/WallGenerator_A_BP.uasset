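; WallGenerator_A_BP is an environment prefab that builds a modular wall from a grid of WallReference meshes.
; Its construction script uses nested loops over NumWallsHori and NumWallsVert to add static mesh components at 200-unit steps along local X and Z.
; The outer loop also places a mesh at each column's base, overlapping the inner loop's first piece.
; The event graph holds only disabled placeholder events.
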(event EventBeginPlay)

(event Collision|EventActorBeginOverlap
  (params (OtherActor :type Actor%20Object%20Reference)))

(event EventTick
  (params (DeltaSeconds :type Float%20%28single-precision%29)))

(fn ConstructionScript
  (for _index (range 0 (- (Variables|Default|GetnumWallsHori) 1))
    (bind _returnvalue (AddComponent|AddStaticMeshComponent false (Math|Transform|MakeTransform (Math|Vector|MakeVector (* (Math|Conversions|ToFloat(Integer) _index) 2e+02) 0.0 0.0))))
    (Components|StaticMesh|SetStaticMesh _returnvalue (Variables|Default|GetwallReference))
    (for _index_2 (range 0 (- (Variables|Default|GetnumWallsVert) 1))
      (bind _returnvalue_2 (AddComponent|AddStaticMeshComponent false (Math|Transform|MakeTransform (Math|Vector|MakeVector (* (Math|Conversions|ToFloat(Integer) _index) 2e+02) 0.0 (* (Math|Conversions|ToFloat(Integer) _index_2) 2e+02)))))
      (Components|StaticMesh|SetStaticMesh _returnvalue_2 (Variables|Default|GetwallReference)))))