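; Prototype floor-style button that opens and closes a referenced door when the player's controlled pawn enters or leaves it.
; Overlapping the trigger plays a timeline that moves the button mesh along Z.
; The timeline's Update output also feeds a short delay before calling OpenTheDoor on the door reference.
; Ending overlap with the actor calls CloseTheDoor immediately, without reversing the button animation.
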(event OnComponentBeginOverlap(trigger)
  (params (OverlappedComponent :type Primitive%20Component%20Object%20Reference) (OtherActor :type Actor%20Object%20Reference) (OtherComp :type Primitive%20Component%20Object%20Reference) (OtherBodyIndex :type Integer) (bFromSweep :type Boolean) (SweepResult :type Hit%20Result%20Structure%20%28by%20ref%29))
  (if (== OtherActor (Pawn|GetControlledPawn (Game|GetPlayerController 0)))
    (bind _buttonlocation (Timeline|buttonMovement Play)
      (:Update
        (Transformation|SetRelativeLocation (Variables|Default|GetButton_01) (Math|Vector|MakeVector 0.0 0.0 _buttonlocation) false false)
        (Utilities|FlowControl|Delay 0.8)
        (Default|OpentheDoor (Variables|Default|Getdoor_Ref))))))

(event Collision|EventActorBeginOverlap
  (params (OtherActor :type Actor%20Object%20Reference)))

(event EventTick
  (params (DeltaSeconds :type Float%20%28single-precision%29)))

(event Collision|EventActorEndOverlap
  (params (OtherActor :type Actor%20Object%20Reference))
  (if (== OtherActor (Pawn|GetControlledPawn (Game|GetPlayerController 0)))
    (Default|ClosetheDoor (Variables|Default|Getdoor_Ref))))

(fn ConstructionScript)