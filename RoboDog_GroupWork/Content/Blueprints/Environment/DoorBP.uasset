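; Sliding door actor with a status light that shows green when open and red when closed.
; Open and close events set IsOpen, swap the light material and both point light colors, then slide the door mesh along its local Y axis via separate timelines.
; Each timeline has a DoOnce gate that resets on finish, blocking restarts mid-motion.
; The construction script defaults the light material to red, and BeginPlay opens the door if IsOpen is set.
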(event Custom|openTheDoor
  (Variables|Default|SetisOpen true)
  (Rendering|Material|SetMaterial (Variables|Default|GetWindowDoor_Light) 0 (Variables|Default|GetgreenLight_ref))
  (Rendering|Components|Light|SetLightColor (Variables|Default|GetPointLight) (Math|Conversions|ToLinearColor(Color) (Variables|Default|Getgreen_Ref)) true)
  (Rendering|Components|Light|SetLightColor (Variables|Default|GetPointLight1) (Math|Conversions|ToLinearColor(Color) (Variables|Default|Getgreen_Ref)) true)
  (Utilities|FlowControl|DoOnce false :!label _label
    (:Completed
      (bind _translatedoor (Timeline|Timeline_0 PlayFromStart)
        (:Update
          (Transformation|SetRelativeLocation (Variables|Default|GetWindowDoor_Door) (Math|Vector|MakeVector 0.0 _translatedoor 0.0) false false))
        (:Finished
          (goto _label Reset))))))

(event Custom|closeTheDoor
  (Variables|Default|SetisOpen false)
  (Rendering|Material|SetMaterial (Variables|Default|GetWindowDoor_Light) 0 (Variables|Default|GetredLight_ref))
  (Rendering|Components|Light|SetLightColor (Variables|Default|GetPointLight) (Math|Conversions|ToLinearColor(Color) (Variables|Default|Getred_Ref)) true)
  (Rendering|Components|Light|SetLightColor (Variables|Default|GetPointLight1) (Math|Conversions|ToLinearColor(Color) (Variables|Default|Getred_Ref)) true)
  (Utilities|FlowControl|DoOnce false :!label _label
    (:Completed
      (bind _translatedoor (Timeline|Timeline_1 PlayFromStart)
        (:Update
          (Transformation|SetRelativeLocation (Variables|Default|GetWindowDoor_Door) (Math|Vector|MakeVector 0.0 _translatedoor 0.0) false false))
        (:Finished
          (goto _label Reset))))))

(event EventBeginPlay
  (if (Variables|Default|GetisOpen)
    (CallFunction|OpentheDoor)))

(fn ConstructionScript
  (Rendering|Material|SetMaterial (Variables|Default|GetWindowDoor_Light) 0 (Variables|Default|GetredLight_ref)))