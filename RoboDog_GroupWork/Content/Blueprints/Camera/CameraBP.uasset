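; Room-aware camera actor that becomes the player's view target and follows the main character from room to room.
; Each tick it finds the overlapped Room_BaseBP flagged as current, then targets the midpoint between the character's CamPosBox and that room's CameraTransformBox, using the room box's rotation with a fixed offset.
; It eases its root toward that target with TInterpTo.
; SetCharRef switches the followed character, and SetRoomRef sets the room externally.
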(event Custom|SetRoomRef
  (params (NewParam :type Room%20Base%20BP%20Object%20Reference))
  (Variables|Default|SetRoomRef NewParam))

(event EventBeginPlay
  (Game|Player|SetViewTargetwithBlend (Game|GetPlayerController 0) self 0.0 "VTBlend_Linear" 0.0 false)
  (bind _asmain_character_bp (Utilities|Casting|CastToMainCharacterBP (Game|GetPlayerCharacter 0)))
  (bind _output_get (Variables|Default|SetCharRef _asmain_character_bp))
  (Variables|Default|SetControlledCharPos (Transformation|GetWorldLocation (Variables|/Script/Engine.Character|GetCapsuleComponent _output_get))))

(event EventTick
  (params (DeltaSeconds :type Float%20%28single-precision%29))
  (Utilities|FlowControl|Sequence
    (:then_0
      (CallFunction|GetRoomTransform))
    (:then_1
      (CallFunction|SetFutureTransform))
    (:then_2
      (CallFunction|HandleLerping DeltaSeconds))))

(fn ConstructionScript)

(fn SetCharRef
  (params (CharRef :type Main%20Character%20BP%20Object%20Reference))
  (bind _output_get (Variables|Default|SetCharRef CharRef))
  (Variables|Default|SetControlledCharPos (Transformation|GetWorldLocation (Variables|/Game/Blueprints/Character/MainCharacterBP.MainCharacterBP_C|GetCamPosBox _output_get)))
  (Game|Player|SetViewTargetwithBlend (Game|GetPlayerController 0) self 0.0 "VTBlend_Linear" 0.0 false))

(fn HandleLerping
  (params (InputPin :type Float%20%28single-precision%29))
  (if true
    (Transformation|SetWorldTransform (Variables|Default|GetDefaultSceneRoot) (Class|KismetMathLibrary|TInterpto (Transformation|GetWorldTransform (Variables|Default|GetDefaultSceneRoot)) (Variables|Default|GetFutureTransform) InputPin 1.0) false false)))

(fn GetRoomTransform
  (bind _array_element (Utilities|Array|ForEachLoopwithBreak (Collision|GetOverlappingActors (Variables|Default|GetCharRef) "/Game/Blueprints/Environment/RoomBP/Room_BaseBP.Room_BaseBP_C" :!class /Script/Engine.Actor) :!label _label)
    (:LoopBody
      (bind _asroom_base_bp (Utilities|Casting|CastToRoom_BaseBP _array_element))
      (if (Variables|/Game/Blueprints/Environment/RoomBP/Room_BaseBP.Room_BaseBP_C|GetIsCurrentRoom _asroom_base_bp)
        (Variables|Default|SetRoomRef _asroom_base_bp)
        (goto _label Break)))))

(fn SetFutureTransform
  (bind _charref (Variables|Default|GetCharRef))
  (bind _roomref (Variables|Default|GetRoomRef))
  (bind _camposbox (Variables|/Game/Blueprints/Character/MainCharacterBP.MainCharacterBP_C|GetCamPosBox _charref))
  (bind _cameratransformbox (Variables|/Game/Blueprints/Environment/RoomBP/Room_BaseBP.Room_BaseBP_C|GetCameraTransformBox _roomref))
  (bind _returnvalue (Transformation|GetWorldTransform _camposbox))
  (bind _returnvalue_2 (Transformation|GetWorldTransform _cameratransformbox))
  (Variables|Default|SetFutureTransform (Math|Transform|MakeTransform (/ (+ (.location _returnvalue) (.location _returnvalue_2)) 2.0) (Math|Rotator|CombineRotators (.rotation _returnvalue_2) "0,-90.000000, 0") (.scale _returnvalue))))